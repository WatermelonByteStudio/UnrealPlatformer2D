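; Player character for a side-scrolling game, handling Enhanced Input movement, jumping and shooting.
; Movement runs along the X axis only, flipping control rotation to face the input direction.
; Jumping or walking off a ledge jumps the animation instance to its InAir node.
; Shooting spawns a projectile at ShootPos and holds a State.Shooting gameplay tag until a retriggerable delay expires.
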(event Input|EnhancedActionEvents|EnhancedInputActionIA_Jump
  (params (ActionValue :type Boolean) (ElapsedSeconds :type Float%20%28double-precision%29) (TriggeredSeconds :type Float%20%28double-precision%29) (InputAction :type Input%20Action%20Object%20Reference :default "/Game/Input/Actions/IA_Jump.IA_Jump"))
  ;[1 1 1] Input / Movement
  (:Started
    (Character|Jump))
  (:Canceled
    (Character|StopJumping :!label _label))
  (:Completed
    (goto _label)))

(event Input|EnhancedActionEvents|EnhancedInputActionIA_Move
  (params (ActionValue :type Float%20%28double-precision%29) (ElapsedSeconds :type Float%20%28double-precision%29) (TriggeredSeconds :type Float%20%28double-precision%29) (InputAction :type Input%20Action%20Object%20Reference :default "/Game/Input/Actions/IA_Move.IA_Move"))
  ;[1 1 1] Input / Movement
  (Pawn|Input|AddMovementInput "1.000000,0.000000,0.000000" ActionValue false)
  (Pawn|SetControlRotation (Pawn|GetController) (Math|Rotator|SelectRotator "0, 0, 0" "0.000000,180.000000,0.000000" (>= ActionValue 0.0))))

(event Input|EnhancedActionEvents|EnhancedInputActionIA_Shoot
  (params (ActionValue :type Boolean) (ElapsedSeconds :type Float%20%28double-precision%29) (TriggeredSeconds :type Float%20%28double-precision%29) (InputAction :type Input%20Action%20Object%20Reference :default "/Game/Input/Actions/IA_Shoot.IA_Shoot"))
  (bind _self self)
  (bind _shootpos (Variables|Default|GetShootPos))
  ;[1 1 1] Shooting event
  (:Started
    (GameplayTags|AddGameplayTag (Variables|Default|GetGameplayTags) "(TagName=\"State.Shooting\")" :!class /Script/GameplayTags.BlueprintGameplayTagLibrary)
    (Game|SpawnActorfromClass "/Game/Blueprints/Projectiles/BP_Projectile_Base.BP_Projectile_Base_C" (Math|Transform|MakeTransform (Transformation|GetWorldLocation _shootpos) (Transformation|GetWorldRotation _shootpos) "1.000000,1.000000,1.000000") "Undefined" "MultiplyWithRoot" _self (Variables|Default|GetDamage) _self)
    (Utilities|FlowControl|RetriggerableDelay 0.4)
    (GameplayTags|RemoveGameplayTag (Variables|Default|GetGameplayTags) "(TagName=\"State.Shooting\")" :!class /Script/GameplayTags.BlueprintGameplayTagLibrary)))

(event EventBeginPlay
  ;[1 1 1] Begin Play
  (|CallParentFunction)
  (bind _asplayer_controller (Utilities|Casting|CastToPlayerController (Pawn|GetController)))
  (Input|AddMappingContext (PlayerController|LocalPlayerSubsystems|GetEnhancedInputLocalPlayerSubsystem _asplayer_controller) "/Game/Input/IMC_Action.IMC_Action" 0 "(bIgnoreAllPressedKeysUntilRelease=True,bForceImmediately=False,bNotifyUserSettings=False)"))

(event EventOnWalkingOffLedge
  (params (PreviousFloorImpactNormal :type Vector%20%28by%20ref%29 :default "0, 0, 0") (PreviousFloorContactNormal :type Vector%20%28by%20ref%29 :default "0, 0, 0") (PreviousLocation :type Vector%20%28by%20ref%29 :default "0, 0, 0") (TimeDelta :type Float%20%28single-precision%29))
  ;[1 1 1] Input / Movement
  ;;[1 1 1] Falling/Jumping Animation call to the ABP
  (Class|PaperZDAnimInstance|JumptoNode (Variables|/Script/PaperZD.PaperZDAnimationComponent|GetAnimInstance (Variables|Default|GetAnimationComponent)) "InAir" "None"))

(event EventOnJumped
  ;[1 1 1] Input / Movement
  ;;[1 1 1] Falling/Jumping Animation call to the ABP
  (Class|PaperZDAnimInstance|JumptoNode (Variables|/Script/PaperZD.PaperZDAnimationComponent|GetAnimInstance (Variables|Default|GetAnimationComponent)) "InAir" "None"))

(fn ConstructionScript
  (|CallParentFunction))