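; BP_Enemy is an enemy character that damages actors of another faction on contact and handles its own death sequence.
; Capsule overlap runs a faction check and, when it returns false, sends a health change message with the overlap damage to the other actor.
; StartDestroySteps passes the sprite and VFX flipbook to a play-once-and-destroy routine.
; BeginPlay and construction defer to the parent class.
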(event OnComponentBeginOverlap(CapsuleComponent)
  (params (OverlappedComponent :type Primitive%20Component%20Object%20Reference) (OtherActor :type Actor%20Object%20Reference) (OtherComp :type Primitive%20Component%20Object%20Reference) (OtherBodyIndex :type Integer) (bFromSweep :type Boolean) (SweepResult :type Hit%20Result%20Structure%20%28by%20ref%29))
  (bind _bsamefaction_ (CallFunction|CheckforActorFaction OtherActor))
  (if (not _bsamefaction_)
    (Class|BPIActionCharHelper|ApplyHealthChange(Message) OtherActor self (Variables|Default|GetOverlapDamage) "NewEnumerator0")))

(event EventBeginPlay
  (|CallParentFunction))

(event EventStartDestroySteps
  (CallFunction|PFlipbookOnceandDestroy (Variables|Default|GetSprite) self (Variables|Default|GetPFB%20VFX)))

(fn ConstructionScript
  (|CallParentFunction))