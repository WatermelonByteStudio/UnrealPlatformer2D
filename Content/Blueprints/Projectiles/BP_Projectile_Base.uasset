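; Base projectile actor with a Paper2D flipbook, sphere collision and projectile movement, which destroys hostile actors and itself on contact.
; A looping timer projects its location to screen and destroys it once it leaves the viewport horizontally.
; Overlaps use BPI_ActionCharHelper messages to let the Instigator check faction before triggering the target's destroy steps.
; Valid overlaps and any blocking hit play the destroy flipbook, stop movement and remove the projectile.
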(event OnComponentHit(Sphere)
  (params (HitComponent :type Primitive%20Component%20Object%20Reference) (OtherActor :type Actor%20Object%20Reference) (OtherComp :type Primitive%20Component%20Object%20Reference) (NormalImpulse :type Vector :default "0, 0, 0") (Hit :type Hit%20Result%20Structure%20%28by%20ref%29))
  ;[1 1 1] On collisition
  (CallFunction|PFlipbookOnceandDestroy (Variables|Default|GetPaperFlipbook) self (Variables|Default|GetPFB_DestroyVFX))
  (Components|Movement|StopMovementImmediately (Variables|Default|GetProjectileMovement)))

(event OnComponentBeginOverlap(Sphere)
  (params (OverlappedComponent :type Primitive%20Component%20Object%20Reference) (OtherActor :type Actor%20Object%20Reference) (OtherComp :type Primitive%20Component%20Object%20Reference) (OtherBodyIndex :type Integer) (bFromSweep :type Boolean) (SweepResult :type Hit%20Result%20Structure%20%28by%20ref%29))
  (if (Utilities|DoesObjectImplementInterface OtherActor "/Game/Blueprints/Utils/Interfaces/BPI_ActionCharHelper.BPI_ActionCharHelper_C")
    (bind _bsamefaction_ (Class|BPIActionCharHelper|CheckforActorFaction(Message) (Variables|Actor|GetInstigator) OtherActor))
    (if _bsamefaction_
      (Class|BPIActionCharHelper|StartDestroySteps(Message) OtherActor)
      ;[1 1 1] On collisition
      (CallFunction|PFlipbookOnceandDestroy (Variables|Default|GetPaperFlipbook) self (Variables|Default|GetPFB_DestroyVFX))
      (Components|Movement|StopMovementImmediately (Variables|Default|GetProjectileMovement)))))

(event Custom|CE_CheckForScreenOutOfBound
  ;[1 1 1] Check out of bound
  (if (not (Math|Float|InRange(Float) (.x (.ScreenLocation (Class|PlayerController|ProjectWorldLocationtoScreen (Game|GetPlayerController 0) (Transformation|GetActorLocation) false))) 0.0 (.x (Viewport|GetViewportSize))))
    (Actor|DestroyActor)))

(event EventBeginPlay
  ;[1 1 1] Check out of bound
  (Utilities|Time|SetTimerbyEvent (delegate Custom|CE_CheckForScreenOutOfBound) 0.5 true))

(event EventDestroyed)

(fn ConstructionScript)