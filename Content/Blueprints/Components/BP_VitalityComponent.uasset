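; BP_VitalityComponent is an actor component that tracks a health value for its owner.
; On BeginPlay it sets current health to the maximum.
; ProcessValue applies an amount as damage or healing by selecting a sign from the type, clamps the result between zero and max, and returns whether health reached zero.
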(event EventBeginPlay
  (Variables|Default|SetCurrentHealth (Variables|Default|GetMaxHealth)))

(fn ProcessValue
  (params (Value :type Float%20%28double-precision%29) (DamageType :type EDamageType%20Enum :default "NewEnumerator0"))
  (bind _output_get (Variables|Default|SetCurrentHealth (Math|Float|Clamp(Float) (+ (Variables|Default|GetCurrentHealth) (* Value (Utilities|Select :Index DamageType :NewEnumerator0 -1.0 :NewEnumerator1 1.0))) 0.0 (Variables|Default|GetMaxHealth))))
  (return (== _output_get 0.0)))